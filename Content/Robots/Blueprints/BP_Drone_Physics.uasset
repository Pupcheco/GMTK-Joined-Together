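; BP_Drone_Physics is a drone Blueprint that keeps the robot hovering through physics forces on its Box component.
; A BeginPlay Delay loop stands in for Tick, polling each second while docked and running every frame otherwise.
; When undocked, it calls VerticalBoost to add RisingForce below FHoverLevel, then always applies a Z force with a fixed offset.
; Both forces use acceleration change, so they ignore mass.
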(event EventBeginPlay
  (if (Variables|Default|GetisDocked) :!label _label
    (Utilities|FlowControl|Delay 1.0)
    (goto _label)
    (else
      (if (< (|GetDroneZ) (Variables|Default|GetfHoverLevel))
        (|VerticalBoost))
      (Physics|AddForce (Variables|Default|GetBox) (Math|Vector|MakeVector 0.0 0.0 (+ (stale _result) 7.2e+02)) "None" true)
      (Utilities|FlowControl|Delay 0.0)
      (goto _label))))

(event Collision|EventActorBeginOverlap
  (params (OtherActor :type Actor%20Object%20Reference)))

(event EventTick
  (params (DeltaSeconds :type Float%20%28single-precision%29)))

(fn ConstructionScript)