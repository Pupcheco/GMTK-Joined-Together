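; Pylon Blueprint that stores power and switches a linked ToActivate object on and off.
; GeneratePower calls raise Power, while Tick constantly drains it, both through delta-time-scaled macros.
; The target receives an activate message at full charge and a deactivate message only once power runs low, giving hysteresis.
; The light snaps between off and max intensity at half power, as its Lerp alpha is fixed at zero.
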(event `self.ReceiveTick`
  (params (DeltaSeconds :type "Float (single-precision)"))
  (bind _light (`self.Light`))
  (bind _toactivate (`self.ToActivate`))
  (bind _output_get (set `self.Power` (`self.M_DecayPower` (`self.Power`) (`self.PowerDecay`))))
  ;[1 1 1] Adjust Lights
  (if (< _output_get 0.5)
    (`LightComponent.SetIntensity` _light (`KismetMathLibrary.Lerp` 0.0 (`self.Max Light Intensity`)))
    (else
      (`LightComponent.SetIntensity` _light (`self.Max Light Intensity`))))
  (if (< _output_get 0.2)
    (if (`self.Activated`)
      (if (!= _toactivate null)
        (message `/Game/Robots/Blueprints/I_Activatable.Deactivate Object` _toactivate)
        (set `self.Activated` false)))))

(event `/Game/Robots/Blueprints/I_Generator.Generate Power`
  (bind _toactivate (`self.ToActivate`))
  (bind _output_get (set `self.Power` (`self.M_GeneratePower` (`self.Power`) (`self.PowerGrowth`))))
  (if (>= (`KismetMathLibrary.FMin` _output_get 1.0) 1.0)
    (if (not (`self.Activated`))
      (if (!= _toactivate null)
        (message `/Game/Robots/Blueprints/I_Activatable.Activate Object` _toactivate)
        (set `self.Activated` true)))))

(fn `UserConstructionScript`)