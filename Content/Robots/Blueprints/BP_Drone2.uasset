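; BP_Drone2 is a drone actor that continuously bobs up and down in place.
; BeginPlay runs a Hover graph, then loops back through a zero-length Delay to repeat it each frame without using Tick.
; Hover keeps X and Y and sets Z by lerping LowAlt to HighAlt with a sine of game time.
; The raw sine alpha spans -1 to 1, so the motion also extends beyond LowAlt.
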(event `self.ReceiveBeginPlay`
  (`self.K2_SetActorLocation` self (`KismetMathLibrary.MakeVector` (.x (`self.K2_GetActorLocation` self)) (.y (`self.K2_GetActorLocation` self)) (`KismetMathLibrary.Lerp` (`self.Low Alt`) (`self.High Alt`) (`KismetMathLibrary.Sin` (* (`KismetSystemLibrary.GetGameTimeInSeconds`) 1.0)))) false false :!label _label)
  (`KismetSystemLibrary.Delay` 0.0)
  (goto _label))

(fn `UserConstructionScript`)