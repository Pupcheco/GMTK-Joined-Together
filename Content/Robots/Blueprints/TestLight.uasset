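; TestLight is a test Blueprint for a power-driven light whose brightness follows a stored Power value.
; The GeneratePower event grows Power through a macro using frame delta time and a PowerMax cap.
; Tick drains Power through a decay macro clamped between zero and one.
; It then lerps intensity using a further decayed value, or applies maximum intensity at full power.
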(event `self.ReceiveTick`
  (params (DeltaSeconds :type "Float (single-precision)"))
  (bind _light (`self.Light`))
  (bind _normalized_power (`self.M_DecayPower` (`self.Power`) (`self.PowerDecay`)))
  (bind _output_get (set `self.Power` _normalized_power))
  ;[1 1 1] Adjust Lights
  (if (< _output_get 1.0)
    (`LightComponent.SetIntensity` _light (`KismetMathLibrary.Lerp` 0.0 (`self.MaxLightIntensity`) _normalized_power))
    (else
      (`LightComponent.SetIntensity` _light (`self.MaxLightIntensity`)))))

(event `/Game/Robots/Blueprints/I_Generator.Generate Power`
  (set `self.Power` (`self.M_GeneratePower` (`self.Power`) (`self.PowerGrowth`))))

(fn `UserConstructionScript`)