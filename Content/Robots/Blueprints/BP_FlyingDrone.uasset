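; BP_FlyingDrone is a flying robot drone that toggles between hovering and being docked to whoever interacts with it.
; While undocked, a per-frame Delay loop runs the Hover macro, bobbing altitude with a game-time sine.
; Interacting either detaches it and resumes hovering, or plays a sound, lerps it toward the interactor's offset point with sweep, then attaches it.
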(event `self.ReceiveBeginPlay`
  (if (not (`self.isDocked`)) :!label _label
    ;[1 1 1] Hover Routine
    (`self.K2_SetActorLocation` self (`KismetMathLibrary.MakeVector` (.x (`self.K2_GetActorLocation` self)) (.y (`self.K2_GetActorLocation` self)) (`KismetMathLibrary.Lerp` (`self.Low Alt`) (`self.High Alt`) (`KismetMathLibrary.Sin` (* (`KismetSystemLibrary.GetGameTimeInSeconds`) 1.0)))) false false)
    (`KismetSystemLibrary.Delay` 0.0)
    (goto _label)))

(event `/Game/Interactables/InteractableInterface.Interact with Object`
  (params (Interactor :type "Actor Object Reference"))
  (bind _returnvalue (`self.K2_GetActorLocation`))
  (bind _returnvalue_2 (+ (`self.K2_GetActorLocation` Interactor) (`self.Docking Offset`)))
  (if (`self.isDocked`)
    ;[1 1 1] Undock the Drone
    (set `self.isDocked` false)
    (`self.K2_DetachFromActor` "KeepWorld" "KeepWorld" "KeepWorld")
    (goto _label)
    (else
      ;[1 1 1] Dock the Drone
      (`GameplayStatics.PlaySoundAtLocation` "/Game/StarterContent/Audio/Collapse01.Collapse01" _returnvalue (struct) 1.0 1.0 0.0 null null null)
      (set `self.Docked Percent` 0.0)
      (while (and (> (`KismetMathLibrary.Vector_DistanceSquared` _returnvalue _returnvalue_2) (`self.Docked Threshold`)) (< (`KismetMathLibrary.FMin` (`self.Docked Percent`) 1.0) 1.0))
        (bind _output_get (set `self.Docked Percent` (`KismetMathLibrary.FMin` (+ (`self.Docked Percent`) (* (`GameplayStatics.GetWorldDeltaSeconds`) 0.001)) 1.0)))
        (`self.K2_SetActorLocation` (`KismetMathLibrary.VLerp` _returnvalue _returnvalue_2 _output_get) true)
        (`KismetSystemLibrary.Delay` 0.0))
      (set `self.isDocked` true)
      (`self.K2_AttachToActor` Interactor "None" "KeepWorld" "SnapToTarget" "KeepWorld"))))

(fn `UserConstructionScript`)