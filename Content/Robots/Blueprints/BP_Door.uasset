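; Door actor that swings its Door component open and closed through a 90-degree yaw in response to ActivateObject and DeactivateObject.
; Each event steps a DoorOpen alpha by delta time and OpenCloseSpeed, lerps the rotation, and repeats through a zero-length Delay instead of Tick or a Timeline.
; The closing loop also exits only at fully open, so it keeps running once closed.
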(event `/Game/Robots/Blueprints/I_Activatable.Activate Object`
  (bind _output_get (set `self.DoorOpen` (`KismetMathLibrary.FMin` (+ (`self.DoorOpen`) (* (`GameplayStatics.GetWorldDeltaSeconds`) (`self.OpenCloseSpeed`))) 1.0) :!label _label))
  (`SceneComponent.K2_SetRelativeRotation` (`self.Door`) (`KismetMathLibrary.MakeRotator` 0.0 0.0 (`KismetMathLibrary.Lerp` 0.0 90.0 _output_get)) false false)
  (if (not (>= (`self.DoorOpen`) 1.0))
    (`KismetSystemLibrary.Delay` 0.0)
    (goto _label)))

(event `/Game/Robots/Blueprints/I_Activatable.Deactivate Object`
  (bind _output_get (set `self.DoorOpen` (`KismetMathLibrary.FMax` (- (`self.DoorOpen`) (* (`GameplayStatics.GetWorldDeltaSeconds`) (`self.OpenCloseSpeed`)))) :!label _label_2))
  (`SceneComponent.K2_SetRelativeRotation` (`self.Door`) (`KismetMathLibrary.MakeRotator` 0.0 0.0 (`KismetMathLibrary.Lerp` 0.0 90.0 _output_get)) false false)
  (if (not (>= (`self.DoorOpen`) 1.0))
    (`KismetSystemLibrary.Delay` 0.0)
    (goto _label_2)))

(fn `UserConstructionScript`)